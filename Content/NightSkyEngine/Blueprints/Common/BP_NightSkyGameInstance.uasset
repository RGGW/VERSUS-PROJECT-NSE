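; BP_NightSkyGameInstance is the game instance Blueprint for NightSkyEngine, handling login, online session hosting and replay list delivery.
; On Init it calls Login after a short delay.
; HostSession creates a two-connection, non-LAN session through the NSE session subsystem when the instance is host.
; Completed replay searches go to the first WBP_ReplayMenu widget found, only when the player controller is a BP_MenuPlayerController.
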(event `HostSession`
  (if (`self.IsHost`)
    (`NSESessionSubsystem.CreateSession` (subsystem `NSESessionSubsystem`) 2 false)))

(event `self.BP_OnFindReplaysComplete`
  (params (AllReplays :type "Array of ReplaySaveInfo Object Reference (by ref)"))
  (cast `/Game/NightSkyEngine/Blueprints/Menu/BP_MenuPlayerController` (`GameplayStatics.GetPlayerController` 0))
  (bind _foundwidgets (`WidgetBlueprintLibrary.GetAllWidgetsOfClass` "/Game/NightSkyEngine/UI/Replay/WBP_ReplayMenu.WBP_ReplayMenu_C" false))
  (`/Game/NightSkyEngine/UI/Replay/WBP_ReplayMenu.OnFindReplays` (`|GetArrayItem` _foundwidgets) AllReplays))

(event `self.ReceiveInit`
  (`KismetSystemLibrary.Delay` 0.2)
  (`self.Login`))